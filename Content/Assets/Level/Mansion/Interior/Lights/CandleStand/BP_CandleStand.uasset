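; BP_CandleStand is a candle stand prop for the mansion interior with an animated point of candlelight.
; On BeginPlay, the AdjustCandle timeline starts at a time offset derived from the mesh's world X and Z, so stands in different places animate out of sync.
; Each update feeds AffectLight, which sets CandleLight's intensity scaled by CandleBrightness, its color, and its position offset from LightLocation.
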(event `self.ReceiveBeginPlay`
  (bind (_returnvalue_x _returnvalue_y _returnvalue_z) (`KismetMathLibrary.BreakVector` (`SceneComponent.K2_GetComponentLocation` (`self.StaticMesh`))))
  (`|ExecutionSequence`
    (:`then_0`
      (bind (_direction _brightness _color _position) (`Timeline|AdjustCandle` :`NewTime` (mod (+ (`KismetMathLibrary.Square` _returnvalue_x) (`KismetMathLibrary.Square` _returnvalue_z)) 2.5) :!via `SetNewTime` :!label _label)
        (:`Update`
          (`self.AffectLight` _brightness _color _position))))
    (:`then_1`
      (goto _label))))

(fn `AffectLight`
  (params (NewBrightness :type "Float (double-precision)") (NewLightColor :type "LinearColor Structure") (NewPosition :type "Vector Structure"))
  (bind _candlelight (`self.CandleLight`))
  (`LightComponent.SetIntensity` _candlelight (* NewBrightness (`self.CandleBrightness`)))
  (`LightComponent.SetLightColor` _candlelight NewLightColor true)
  (`SceneComponent.K2_SetRelativeLocation` _candlelight (+ (`self.LightLocation`) NewPosition) false true))

(fn `UserConstructionScript`)