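; BP_Ghost is the ghost character Blueprint, exposing name and action labels to interactors by type.
; On BeginPlay it creates an interaction menu widget for its player controller, set to the Runner interactor type, and stores it as InteractPrompt.
; Chasers get "Terrorize" and "Paralyze" as primary and secondary action labels, Runners get empty ones.
; GetName returns CharacterName for every interactor type.
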(event `self.ReceiveBeginPlay`
  (`self.InitializeUI`))

(fn `GetName`
  (params (InteractorType :type "EInteractorType Enum" :default "Runner"))
  (returns (ReturnValue :type Text))
  (switch `EInteractorType` InteractorType
    (:`Runner`
      _)
    (:`Chaser`
      _)
    (:`Ghost`
      _))
  (return (`KismetTextLibrary.Conv_StringToText` (`self.CharacterName`))))

(fn `GetPrimaryAction`
  (params (InteractorType :type "EInteractorType Enum" :default "Runner"))
  (returns (ReturnValue :type Text))
  (switch `EInteractorType` InteractorType
    (:`Runner`
      (return ""))
    (:`Chaser`
      (return "Terrorize"))))

(fn `GetSecondaryAction`
  (params (InteractorType :type "EInteractorType Enum" :default "Runner"))
  (returns (ReturnValue :type Text))
  (switch `EInteractorType` InteractorType
    (:`Runner`
      (return ""))
    (:`Chaser`
      (return "Paralyze"))))

(fn `InitializeUI`
  (bind _asplayer_controller (cast `PlayerController` (`self.GetController`)))
  (bind _returnvalue (`|CreateWidget` "/Game/Blueprints/UI/Widgets/Interaction/BPW_InteractionMenu.BPW_InteractionMenu_C" _asplayer_controller))
  (set `self.InteractPrompt` _returnvalue))

(fn `UserConstructionScript`
  (`parent.UserConstructionScript`))