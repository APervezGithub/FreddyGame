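; BP_CameraTracer manages the on-screen interaction prompt for a camera tracer through show, update and hide events.
; Showing creates a BPW_InteractionMenu for the tracer's interactor type, passes it the target interface and component, refreshes it and adds it to the viewport.
; Update refreshes the stored widget and hide removes it from its parent, both only when it is valid.
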(event `self.ShowInteractPrompt`
  (params (Interface :type "InteractInterface Interface (by ref)") (Component :type "InteractableComponent Object Reference"))
  (bind _returnvalue (`|CreateWidget` "/Game/Blueprints/UI/Widgets/Interaction/BPW_InteractionMenu.BPW_InteractionMenu_C" null (`self.TracerInteractorType`)))
  (bind _output_get (set `self.InteractPrompt` _returnvalue))
  (`/Engine/EditorBlueprintResources/StandardMacros.IsValid` _output_get
    (:`Is Valid`
      (`/Game/Blueprints/UI/Widgets/Interaction/BPW_InteractionMenu.SetInterface` _output_get Interface)
      (`/Game/Blueprints/UI/Widgets/Interaction/BPW_InteractionMenu.SetComponent` _output_get Component)
      (`/Game/Blueprints/UI/Widgets/Interaction/BPW_InteractionMenu.UpdatePrompt` _output_get)
      (`UserWidget.AddToViewport` _output_get 0))))

(event `self.UpdateInteractPrompt`
  (bind _interactprompt (`self.InteractPrompt`))
  (`/Engine/EditorBlueprintResources/StandardMacros.IsValid` _interactprompt
    (:`Is Valid`
      (`/Game/Blueprints/UI/Widgets/Interaction/BPW_InteractionMenu.UpdatePrompt` _interactprompt))))

(event `self.HideInteractPrompt`
  (bind _interactprompt (`self.InteractPrompt`))
  (`/Engine/EditorBlueprintResources/StandardMacros.IsValid` _interactprompt
    (:`Is Valid`
      (`Widget.RemoveFromParent` _interactprompt))))