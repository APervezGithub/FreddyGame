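; BP_LoadingController is the player controller for the startup loading screen shown before the main menu.
; On BeginPlay it shows the cursor, locks input to UI only and creates the BPW_MainLoading widget for the local player.
; Login, session-creation and friends-list events advance that widget's loading state.
; OpenMainMenu opens the MainMenu level as a listen server and removes the widget.
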(event `self.ReceiveBeginPlay`
  (set `self.bShowMouseCursor` true)
  (`self.ShowLoading`)
  (`WidgetBlueprintLibrary.SetInputMode_UIOnlyEx` self null "LockInFullscreen"))

(event `self.SetLoggedIn`
  (`/Game/Blueprints/UI/Menus/LoadingMenu/BPW_MainLoading.UpdateLoading` (`self.MainLoadingRef`) "NewEnumerator3"))

(event `self.SetSessionCreated`
  (`/Game/Blueprints/UI/Menus/LoadingMenu/BPW_MainLoading.UpdateLoading` (`self.MainLoadingRef`) "NewEnumerator2"))

(event `self.SetFriendsListInitiallyRead`
  (`/Game/Blueprints/UI/Menus/LoadingMenu/BPW_MainLoading.UpdateLoading` (`self.MainLoadingRef`) "NewEnumerator4"))

(event `self.OpenMainMenu`
  (`GameplayStatics.OpenLevel` "MainMenu" true "?listen")
  (`self.HideLoading`))

(fn `HideLoading`
  (`Widget.RemoveFromParent` (`self.MainLoadingRef`)))

(fn `ShowLoading`
  (if (`self.IsLocalPlayerController`)
    (bind _returnvalue (`|CreateWidget` "/Game/Blueprints/UI/Menus/LoadingMenu/BPW_MainLoading.BPW_MainLoading_C"))
    (bind _output_get (set `self.MainLoadingRef` _returnvalue))
    (`UserWidget.AddToViewport` _output_get 0)))

(fn `UserConstructionScript`)