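; BP_MenuController is the player controller for the main menu, setting up cursor, input and UI when play begins.
; It shows the mouse, switches to UI-only input and, for a local controller, adds a BPW_MainContainer widget to the viewport.
; It then has BP_EOSGameInstance create a notification container.
; It also forwards friend updates to the menu widget and can remove that widget from the screen.
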(event `self.ReceiveBeginPlay`
  (set `self.bShowMouseCursor` true)
  (`WidgetBlueprintLibrary.SetInputMode_UIOnlyEx` self null "LockInFullscreen")
  (`self.ShowMainMenu`)
  (bind _asbp_eosgame_instance (cast `/Game/Blueprints/Game/BP_EOSGameInstance` (`GameplayStatics.GetGameInstance`)))
  (`/Game/Blueprints/Game/BP_EOSGameInstance.CreateNotificationContainer` _asbp_eosgame_instance))

(event `self.UpdateFriends`
  (`/Game/Blueprints/UI/Menus/MainMenu/BPW_MainContainer.UpdateFriends` (`self.MainMenuRef`)))

(fn `HideMainMenu`
  (`Widget.RemoveFromParent` (`self.MainMenuRef`)))

(fn `ShowMainMenu`
  (if (`self.IsLocalPlayerController`)
    (bind _returnvalue (`|CreateWidget` "/Game/Blueprints/UI/Menus/MainMenu/BPW_MainContainer.BPW_MainContainer_C"))
    (bind _output_get (set `self.MainMenuRef` _returnvalue))
    (`UserWidget.AddToViewport` _output_get 0)))

(fn `UserConstructionScript`)