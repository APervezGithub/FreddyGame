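; BP_TestInteractable is a test interactable that prints debug messages to show when interaction and focus events fire.
; Separate events report the interaction type on the server, calling client and all clients, with the first two also naming the caller.
; Focus start and end print brief messages.
; Name, primary action and secondary action getters return placeholder text for the Runner or Chaser interactor type.
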(event `InteractInterface.OnInteract_BP`
  (params (Caller :type "Actor Object Reference") (InteractionType :type "EInteractionType Enum" :default "Primary"))
  (`KismetSystemLibrary.PrintString` (`KismetStringLibrary.Concat_StrStr` (`KismetSystemLibrary.GetDisplayName` Caller) " uses " (`|GetEnumeratorNameAsString` InteractionType) " interaction on server") true true (struct :`G` 0.66 :`B` 1.0 :`A` 1.0) 3.0))

(event `InteractInterface.StartFocus_BP`
  (`KismetSystemLibrary.PrintString` "focused" true true (struct :`G` 0.66 :`B` 1.0 :`A` 1.0) 0.2))

(event `InteractInterface.CallerOnInteract_BP`
  (params (Caller :type "Actor Object Reference") (InteractionType :type "EInteractionType Enum" :default "Primary"))
  (`KismetSystemLibrary.PrintString` (`KismetStringLibrary.Concat_StrStr` (`KismetSystemLibrary.GetDisplayName` Caller) " uses " (`|GetEnumeratorNameAsString` InteractionType) " interaction on calling client") true true (struct :`G` 0.66 :`B` 1.0 :`A` 1.0) 3.0))

(event `InteractInterface.EndFocus_BP`
  (`KismetSystemLibrary.PrintString` "unfocused" true true (struct :`G` 0.66 :`B` 1.0 :`A` 1.0) 0.2))

(event `self.ReactToInteract_BP`
  (params (InteractionType :type "EInteractionType Enum" :default "Primary"))
  (`KismetSystemLibrary.PrintString` (`KismetStringLibrary.Concat_StrStr` (`|GetEnumeratorNameAsString` InteractionType) " interaction for all clients ") true true (struct :`G` 0.66 :`B` 1.0 :`A` 1.0) 3.0))

(fn `GetName`
  (params (InteractorType :type "EInteractorType Enum" :default "Runner"))
  (returns (ReturnValue :type Text))
  (switch `EInteractorType` InteractorType
    (:`Runner`
      (return "Runner Name"))
    (:`Chaser`
      (return "Chaser Name"))))

(fn `GetPrimaryAction`
  (params (InteractorType :type "EInteractorType Enum" :default "Runner"))
  (returns (ReturnValue :type Text))
  (switch `EInteractorType` InteractorType
    (:`Runner`
      (return "Runner Primary Action"))
    (:`Chaser`
      (return "Chaser Primary Action"))))

(fn `GetSecondaryAction`
  (params (InteractorType :type "EInteractorType Enum" :default "Runner"))
  (returns (ReturnValue :type Text))
  (switch `EInteractorType` InteractorType
    (:`Runner`
      (return "Runner Secondary Action"))
    (:`Chaser`
      (return "Chaser Secondary Action"))))

(fn `UserConstructionScript`)