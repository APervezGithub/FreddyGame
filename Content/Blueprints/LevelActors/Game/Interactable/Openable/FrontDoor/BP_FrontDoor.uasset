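; BP_FrontDoor is an interactable front door that Runners and Chasers can open and close, while Ghosts get no prompt.
; Primary interaction locks further input, flips Toggled, drives ABP_FrontDoor's IsOpen and swaps the closed collision box for left and right boxes.
; The replication callback reapplies animation and collision.
; SetHasOpened and SetHasClosed re-enable interaction when the state matches; door audio is only a debug print.
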(event `self.ReceiveTick`
  (params (DeltaSeconds :type "Float (single-precision)")))

(event `InteractInterface.OnInteract_BP`
  (params (Caller :type "Actor Object Reference") (InteractionType :type "EInteractionType Enum" :default "Primary") (InteractorType :type "EInteractorType Enum" :default "Runner"))
  (switch `EInteractionType` InteractionType
    (:`Primary`
      (`InteractableComponent.SetCanInteract` (`self.InteractableRef`) "Primary" false)
      (`self.Toggle`)
      (`self.OpenDoor`)
      (`self.ToggleCollision`))))

(event `self.ReactToInteract_BP`
  (params (InteractionType :type "EInteractionType Enum" :default "Primary") (InteractorType :type "EInteractorType Enum" :default "Runner"))
  (switch `EInteractionType` InteractionType
    (:`Primary`
      (`KismetSystemLibrary.PrintString` "Play gate audio" true false (struct :`R` 1.0 :`G` 0.736359 :`A` 1.0) 1.0))))

(event `self.OnRep_Toggled_BP`
  (`self.OpenDoor`)
  (`self.ToggleCollision`))

(fn `GetName`
  (params (InteractorType :type "EInteractorType Enum" :default "Runner"))
  (returns (ReturnValue :type Text))
  (return "Front Door"))

(fn `GetPrimaryAction`
  (params (InteractorType :type "EInteractorType Enum" :default "Runner"))
  (returns (ReturnValue :type Text))
  (switch `EInteractorType` InteractorType
    (:`Runner`
      _)
    (:`Chaser`
      _)
    (:`Ghost`
      (return "")))
  (if (`self.Toggled`)
    (return "Close Door")
    (else
      (return "Open Door"))))

(fn `GetSecondaryAction`
  (params (InteractorType :type "EInteractorType Enum" :default "Runner"))
  (returns (ReturnValue :type Text))
  (return ""))

(fn `OpenDoor`
  (bind _asabp_front_door (cast `/Game/Assets/Level/Mansion/Walls/FullWall/DoubleDoorWall/ABP_FrontDoor` (`SkeletalMeshComponent.GetAnimInstance` (`self.SkeletalMesh`))))
  (set `/Game/Assets/Level/Mansion/Walls/FullWall/DoubleDoorWall/ABP_FrontDoor.IsOpen` (`self.Toggled`) _asabp_front_door))

(fn `SetHasClosed`
  (if (not (`self.Toggled`))
    (`InteractableComponent.SetCanInteract` (`self.InteractableRef`) "Primary" true)))

(fn `SetHasOpened`
  (if (`self.Toggled`)
    (`InteractableComponent.SetCanInteract` (`self.InteractableRef`) "Primary" true)))

(fn `ToggleCollision`
  (bind _closedbox (`self.ClosedBox`))
  (bind _leftbox (`self.LeftBox`))
  (bind _rightbox (`self.RightBox`))
  (if (`self.Toggled`)
    (`PrimitiveComponent.SetCollisionEnabled` _closedbox "NoCollision")
    (`PrimitiveComponent.SetCollisionEnabled` _leftbox "QueryAndPhysics")
    (`PrimitiveComponent.SetCollisionEnabled` _rightbox "QueryAndPhysics")
    (else
      (`PrimitiveComponent.SetCollisionEnabled` _closedbox "QueryAndPhysics")
      (`PrimitiveComponent.SetCollisionEnabled` _leftbox "NoCollision")
      (`PrimitiveComponent.SetCollisionEnabled` _rightbox "NoCollision"))))

(fn `UserConstructionScript`)